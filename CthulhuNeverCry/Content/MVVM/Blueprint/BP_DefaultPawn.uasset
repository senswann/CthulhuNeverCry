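; Default pawn that drives a timed fill-and-produce counter for one selected MVVM button viewmodel, such as Cultist, Ghoul or Shambler.
; ChangeId picks the viewmodel from VMOverlay and copies its count, quantity and limits into local variables.
; A looping timer, paused at BeginPlay, raises Count, writing progress and completed Quantity back to the viewmodel until the maximum.
; PlayTimer toggles that timer; despite the parameter name, IsPause=true resumes it.
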(event `self.ReceiveBeginPlay`
  (bind _returnvalue (`KismetSystemLibrary.K2_SetTimerDelegate` (delegate `CustomEvent`) 0.1 true))
  (bind _output_get (set `self.EventClick` _returnvalue))
  (`KismetSystemLibrary.K2_PauseTimerHandle` _output_get))

(event `CustomEvent`
  (bind _quantity (`self.Quantity`))
  (bind _vmbutton (`self.VMButton`))
  (if (< (`self.Quantity`) (`self.MaxQuantity`))
    (`self.AddCount` 1)
    (if (>= (`self.Count`) (`self.MaxCount`))
      (bind _output_get (set `self.Count` 0))
      (set `/Game/MVVM/MVVM/VM_Button.Count` (`KismetMathLibrary.Conv_IntToDouble` _output_get) _vmbutton)
      (bind _result (`/Engine/EditorBlueprintResources/StandardMacros.IncrementInt` _quantity)
        (:`  `
          (set `/Game/MVVM/MVVM/VM_Button.Qt` _result _vmbutton)
          (if (not (< _quantity (`self.MaxQuantity`)))
            (`self.PlayTimer` false)))))))

(event `AddCount`
  (params (HpToAdd :type Integer))
  (bind _output_get (set `self.Count` (`KismetMathLibrary.Clamp` (+ HpToAdd (`self.Count`)) 0 (`self.MaxCount`))))
  (set `/Game/MVVM/MVVM/VM_Button.Count` (`KismetMathLibrary.Conv_IntToDouble` _output_get) (`self.VMButton`)))

(event `AddMaxCount`
  (params (MaxHpToAdd :type Integer))
  (bind _output_get (set `self.MaxCount` (+ MaxHpToAdd (`self.MaxCount`))))
  (set `/Game/MVVM/MVVM/VM_Button.MaxCount` (`KismetMathLibrary.Conv_IntToDouble` _output_get) (`self.VMButton`)))

(fn `ChangeId`
  (params (Id :type Name))
  (bind _vmoverlay (`self.VMOverlay`))
  (bind _vmbutton (`self.VMButton`))
  (switch `name` Id
    (:`00`
      (set `self.VMButton` (`/Game/MVVM/MVVM/VM_Overlay.VMCultist` (`self.VMOverlay`))))
    (:`01`
      (set `self.VMButton` (`/Game/MVVM/MVVM/VM_Overlay.VMGhoul` _vmoverlay)))
    (:`02`
      (set `self.VMButton` (`/Game/MVVM/MVVM/VM_Overlay.VMShamblerTent` _vmoverlay)))
    (:`03`
      (set `self.VMButton` (`/Game/MVVM/MVVM/VM_Overlay.VMShambler` _vmoverlay)))
    (:`04`
      (set `self.VMButton` (`/Game/MVVM/MVVM/VM_Overlay.VMHeart` _vmoverlay))))
  (set `self.Count` (`KismetMathLibrary.FTrunc` (`/Game/MVVM/MVVM/VM_Button.Count` _vmbutton)))
  (set `self.MaxCount` (`KismetMathLibrary.FTrunc` (`/Game/MVVM/MVVM/VM_Button.MaxCount` _vmbutton)))
  (set `self.Quantity` (`/Game/MVVM/MVVM/VM_Button.Qt` _vmbutton))
  (set `self.MaxQuantity` (`/Game/MVVM/MVVM/VM_Button.MaxQt` _vmbutton))
  (`self.InitData`))

(fn `InitData`
  (`self.AddCount` 0)
  (`self.AddMaxCount` 0))

(fn `PlayTimer`
  (params (isPause :type Boolean))
  (bind _eventclick (`self.EventClick`))
  (if isPause
    (`KismetSystemLibrary.K2_UnPauseTimerHandle` _eventclick)
    (else
      (`KismetSystemLibrary.K2_PauseTimerHandle` _eventclick))))

(fn `UserConstructionScript`)